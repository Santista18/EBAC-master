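; BP_Pickup_Master is a base pickup actor that the player can collect through interaction.
; Its box overlap registers it as the third-person character's last interactive object and sets a look-at target, while leaving clears look-at.
; Interact, when allowed, calls an empty Body event for children to override, then destroys the actor.
; The construction script loads Item from a data table row, but mesh assignment is disconnected.
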(event `self.Box.OnComponentBeginOverlap`
  (params (OverlappedComponent :type "PrimitiveComponent Object Reference") (OtherActor :type "Actor Object Reference") (OtherComp :type "PrimitiveComponent Object Reference") (OtherBodyIndex :type Integer) (bFromSweep :type Boolean) (SweepResult :type "HitResult Structure (by ref)"))
  ;[0.1388 0.15 0 0.5] Enter/Exit Colision
  (bind _asbp_third_person_character (cast `/Game/ThirdPerson/Blueprints/BP_ThirdPersonCharacter` OtherActor))
  (set `/Game/ThirdPerson/Blueprints/BP_ThirdPersonCharacter.LastInteractiveObject` self _asbp_third_person_character)
  (set `self.CanInteract?` true)
  ; LookAt
  (set `/Game/ThirdPerson/Blueprints/BP_ThirdPersonCharacter.IsLookAt` true _asbp_third_person_character)
  (set `/Game/ThirdPerson/Blueprints/BP_ThirdPersonCharacter.LookAtPosition` (`self.K2_GetActorLocation`) _asbp_third_person_character))

(event `self.Box.OnComponentEndOverlap`
  (params (OverlappedComponent :type "PrimitiveComponent Object Reference") (OtherActor :type "Actor Object Reference") (OtherComp :type "PrimitiveComponent Object Reference") (OtherBodyIndex :type Integer))
  ;[0.1388 0.15 0 0.5] Enter/Exit Colision
  (bind _asbp_third_person_character (cast `/Game/ThirdPerson/Blueprints/BP_ThirdPersonCharacter` OtherActor))
  (set `self.CanInteract?` false)
  ; LookAt
  (set `/Game/ThirdPerson/Blueprints/BP_ThirdPersonCharacter.IsLookAt` false _asbp_third_person_character))

(event `/Game/Blueprints/Interact_Interface.Interact`
  ; Body
  (if (`self.CanInteract?`)
    (`self.Body`)
    (`self.K2_DestroyActor`)
    (`KismetSystemLibrary.PrintString` "Coletada")))

(event `Body`
  ; Body
)

(fn `UserConstructionScript`
  (bind (_datatable _rowname) (break `DataTableRowHandle` (`self.Data Table Row Handle`)))
  (bind _returnvalue (`|GetDataTableRow` _datatable _rowname)
    (:`then`
      (bind _output_get (set `self.Item` _returnvalue)))))