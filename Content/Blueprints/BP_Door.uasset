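; BP_Door is an interactive door that swings open only when its HasKey flag is set.
; A box overlap registers the door as the third-person character's LastInteractiveObject and toggles CanInteract.
; Interact alternates through a FlipFlop between playing and reversing a Timeline that drives the Porta component's yaw, with DoorOpen updated on finish.
; NewFunction and Soma are helper functions that the event graph never calls.
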(event `self.Box.OnComponentBeginOverlap`
  (params (OverlappedComponent :type "PrimitiveComponent Object Reference") (OtherActor :type "Actor Object Reference") (OtherComp :type "PrimitiveComponent Object Reference") (OtherBodyIndex :type Integer) (bFromSweep :type Boolean) (SweepResult :type "HitResult Structure (by ref)"))
  ; Santos is Giant Go Santos
  ;;[0.15 0.1396 0 0.5] Enter Colision
  (bind _asbp_third_person_character (cast `/Game/ThirdPerson/Blueprints/BP_ThirdPersonCharacter` OtherActor))
  (set `/Game/ThirdPerson/Blueprints/BP_ThirdPersonCharacter.LastInteractiveObject` self _asbp_third_person_character)
  (set `self.CanInteract?` true))

(event `self.Box.OnComponentEndOverlap`
  (params (OverlappedComponent :type "PrimitiveComponent Object Reference") (OtherActor :type "Actor Object Reference") (OtherComp :type "PrimitiveComponent Object Reference") (OtherBodyIndex :type Integer))
  ; Santos is Giant Go Santos
  ;;[0.15 0.1396 0 0.5] Exit Colision
  (cast `/Game/ThirdPerson/Blueprints/BP_ThirdPersonCharacter` OtherActor)
  (set `self.CanInteract?` false))

(event `/Game/Blueprints/Interact_Interface.Interact`
  ; Santos is Giant Go Santos
  ;; Interact
  (if (`self.CanInteract?`)
    (`/Engine/EditorBlueprintResources/StandardMacros.FlipFlop`
      (:`A`
        (if (`self.HasKey?`)
          (if (not (`self.DoorOpen?`))
            (`/Engine/EditorBlueprintResources/StandardMacros.IsValid` "BP_Door"
              (:`Is Valid`
                (bind (_direction `_rotação`) (`Timeline|Timeline` :!via `PlayFromStart` :!label _label)
                  (:`Update`
                    _)
                  (:`Finished`
                    (set `self.DoorOpen?` (> `_rotação` 0.0))))
                (`SceneComponent.K2_SetRelativeRotation` (`self.Porta`) (`KismetMathLibrary.MakeRotator` 0.0 0.0 `_rotação`) false false))))))
      (:`B`
        (if (`self.DoorOpen?`)
          (goto _label :!via `ReverseFromEnd`))))))

(fn `NewFunction`
  (returns (NewParam :type Boolean))
  (bind _dooropen_ (`self.DoorOpen?`))
  (if (not _dooropen_)
    (`SceneComponent.K2_AddLocalOffset` (`self.Porta`) (0.0 0.0 0.0) false false)
    (else
      (`KismetSystemLibrary.PrintString` "Precisa de Chave")
      (return _dooropen_))))

(fn `Soma`
  (params (NewParam :type "Float (double-precision)") (NewParam1 :type "Vector Structure"))
  (returns (NewParam2 :type "Vector Structure"))
  (return (* NewParam NewParam1)))

(fn `UserConstructionScript`)